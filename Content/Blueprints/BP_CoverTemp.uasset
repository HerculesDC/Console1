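; BP_CoverTemp is a cover actor that tells the player pawn which of its Front or Back volumes it is overlapping.
; On begin overlap, either volume calls HidePlayer, which stores that volume in BP_PlayerPawn's OverlappingBoxCollision.
; On end overlap, UnhidePlayer clears the reference only if it still points to the exited volume, so moving between overlapping volumes keeps the newer one.
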(event `self.ReceiveActorBeginOverlap`
  (params (OtherActor :type "Actor Object Reference")))

(event `self.Back.OnComponentBeginOverlap`
  (params (OverlappedComponent :type "PrimitiveComponent Object Reference") (OtherActor :type "Actor Object Reference") (OtherComp :type "PrimitiveComponent Object Reference") (OtherBodyIndex :type Integer) (bFromSweep :type Boolean) (SweepResult :type "HitResult Structure (by ref)"))
  (`self.HidePlayer` OtherActor (`self.Back`)))

(event `self.Back.OnComponentEndOverlap`
  (params (OverlappedComponent :type "PrimitiveComponent Object Reference") (OtherActor :type "Actor Object Reference") (OtherComp :type "PrimitiveComponent Object Reference") (OtherBodyIndex :type Integer))
  (`self.UnhidePlayer` OtherActor (`self.Back`)))

(event `HidePlayer`
  (params (OverlappedActor :type "Actor Object Reference") (OverlappingVolume :type "BoxComponent Object Reference"))
  (bind _asbp_player_pawn (cast `/Game/Blueprints/BP_PlayerPawn` OverlappedActor))
  (set `TPSCharacter.OverlappingBoxCollision` OverlappingVolume _asbp_player_pawn))

(event `UnhidePlayer`
  (params (OverlappedActor :type "Actor Object Reference") (OverlappingVolume :type "BoxComponent Object Reference"))
  (bind _asbp_player_pawn (cast `/Game/Blueprints/BP_PlayerPawn` OverlappedActor))
  (if (== (`TPSCharacter.OverlappingBoxCollision` _asbp_player_pawn) OverlappingVolume)
    (set `TPSCharacter.OverlappingBoxCollision` null _asbp_player_pawn)))

(event `self.Front.OnComponentBeginOverlap`
  (params (OverlappedComponent :type "PrimitiveComponent Object Reference") (OtherActor :type "Actor Object Reference") (OtherComp :type "PrimitiveComponent Object Reference") (OtherBodyIndex :type Integer) (bFromSweep :type Boolean) (SweepResult :type "HitResult Structure (by ref)"))
  (`self.HidePlayer` OtherActor (`self.Front`)))

(event `self.Front.OnComponentEndOverlap`
  (params (OverlappedComponent :type "PrimitiveComponent Object Reference") (OtherActor :type "Actor Object Reference") (OtherComp :type "PrimitiveComponent Object Reference") (OtherBodyIndex :type Integer))
  (`self.UnhidePlayer` OtherActor (`self.Front`)))

(fn `UserConstructionScript`)